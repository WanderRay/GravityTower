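; ZoneDeDamage5 is a damage zone that sends the player back to the CheckPoint5 actor on contact.
; When its Collision component is overlapped by a DGCharacterBP, it finds that checkpoint by class and teleports the character to its location with zero rotation.
; It then plays a 2D sound and spawns two particle effects at the character's location.
; Delayed cleanup nodes for both emitters exist but are unconnected.
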(event `self.Collision.OnComponentBeginOverlap`
  (params (OverlappedComponent :type "PrimitiveComponent Object Reference") (OtherActor :type "Actor Object Reference") (OtherComp :type "PrimitiveComponent Object Reference") (OtherBodyIndex :type Integer) (bFromSweep :type Boolean) (SweepResult :type "HitResult Structure (by ref)"))
  ;[1 1 1] Téléportation If Hitten
  (`|ExecutionSequence`
    (:`then_0`
      (bind _asdgcharacter_bp (cast `/Game/DynamicGravityCharacter/Blueprints/Character+MovingWalls/DGCharacterBP` OtherActor))
      (bind _returnvalue (`GameplayStatics.GetActorOfClass` "/Game/DynamicGravityCharacter/Blueprints/ZonesInteractions/CheckPoint5.CheckPoint5_C"))
      (`self.K2_TeleportTo` :`self` _asdgcharacter_bp :`DestLocation` (`self.K2_GetActorLocation` _returnvalue))
      (`GameplayStatics.PlaySound2D` "/Game/DynamicGravityCharacter/SFX/Mifa.Mifa" 1.0 1.0 0.0 null null)
      (`|ExecutionSequence`
        (:`then_0`
          (bind _returnvalue_location (`KismetMathLibrary.BreakTransform` (`self.GetTransform` _asdgcharacter_bp)))
          (bind _returnvalue_2 (`GameplayStatics.SpawnEmitterAtLocation` "/Game/RPGEffects/Particles/P_Mage_MagicSphere.P_Mage_MagicSphere" _returnvalue_location (struct) (0.1 0.1 0.1))))
        (:`then_1`
          (bind _returnvalue_3 (`GameplayStatics.SpawnEmitterAtLocation` "/Game/RPGEffects/Particles/P_Targeting_Player_Movement.P_Targeting_Player_Movement" _returnvalue_location)))))))

(fn `UserConstructionScript`)