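; SuccessBox1 is a puzzle success trigger that, once only, opens three shoji doors when anything overlaps its collision.
; It plays an unlock sound and runs three timelines, each sliding one door found by class along X or Y.
; The offsets add to the current location every update, so travel accumulates per frame.
; It also calls CallCameraPiece1, then after a delay has Receptacle2 call SwitchToCharacter.
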(event `self.Collision.OnComponentBeginOverlap`
  (params (OverlappedComponent :type "PrimitiveComponent Object Reference") (OtherActor :type "Actor Object Reference") (OtherComp :type "PrimitiveComponent Object Reference") (OtherBodyIndex :type Integer) (bFromSweep :type Boolean) (SweepResult :type "HitResult Structure (by ref)"))
  (`self.OuvrirLesPortes`))

(event `OuvrirLesPortes`
  (`/Engine/EditorBlueprintResources/StandardMacros.DoOnce` false
    (:`Completed`
      (`|ExecutionSequence`
        (:`then_0`
          (`GameplayStatics.PlaySound2D` "/Game/DynamicGravityCharacter/SFX/UnlockingSpecialNote.UnlockingSpecialNote" 1.0 1.0 0.0 null null)
          (`|ExecutionSequence`
            (:`then_0`
              (bind _returnvalue (`GameplayStatics.GetActorOfClass` "/Game/DynamicGravityCharacter/Blueprints/ZonesInteractions/ShojiDoor/ShojiDoor1.ShojiDoor1_C"))
              (bind (_direction _1_0) (`Timeline|Timeline_0` :!via `PlayFromStart`)
                (:`Update`
                  (bind (_returnvalue_x _returnvalue_y _returnvalue_z) (`KismetMathLibrary.BreakVector` (`self.K2_GetActorLocation` _returnvalue)))
                  (`self.K2_SetActorLocation` _returnvalue (`KismetMathLibrary.MakeVector` (+ (`KismetMathLibrary.Lerp` 0.0 6.0 _1_0) _returnvalue_x) _returnvalue_y _returnvalue_z) false false))))
            (:`then_1`
              (bind _returnvalue_2 (`GameplayStatics.GetActorOfClass` "/Game/DynamicGravityCharacter/Blueprints/ZonesInteractions/ShojiDoor/ShojiDoor2.ShojiDoor2_C"))
              (bind (_direction_2 _1_0_2) (`Timeline|Timeline_1` :!via `PlayFromStart`)
                (:`Update`
                  (bind (_returnvalue_x_2 _returnvalue_y_2 _returnvalue_z_2) (`KismetMathLibrary.BreakVector` (`self.K2_GetActorLocation` _returnvalue_2)))
                  (`self.K2_SetActorLocation` _returnvalue_2 (`KismetMathLibrary.MakeVector` _returnvalue_x_2 (+ (`KismetMathLibrary.Lerp` 0.0 -6.0 _1_0_2) _returnvalue_y_2) _returnvalue_z_2) false false))))
            (:`then_2`
              (bind _returnvalue_3 (`GameplayStatics.GetActorOfClass` "/Game/DynamicGravityCharacter/Blueprints/ZonesInteractions/ShojiDoor/ShojiDoor3.ShojiDoor3_C"))
              (bind (_direction_3 _1_0_3) (`Timeline|Timeline_2` :!via `PlayFromStart`)
                (:`Update`
                  (bind (_returnvalue_x_3 _returnvalue_y_3 _returnvalue_z_3) (`KismetMathLibrary.BreakVector` (`self.K2_GetActorLocation` _returnvalue_3)))
                  (`self.K2_SetActorLocation` _returnvalue_3 (`KismetMathLibrary.MakeVector` _returnvalue_x_3 (+ (`KismetMathLibrary.Lerp` 0.0 6.0 _1_0_3) _returnvalue_y_3) _returnvalue_z_3) false false))))))
        (:`then_1`
          (`self.CallCameraPiece1`)
          (`KismetSystemLibrary.Delay` 3.0)
          (bind _returnvalue_4 (`GameplayStatics.GetActorOfClass` "/Game/DynamicGravityCharacter/Blueprints/Collectable_Receptacle/Receptacle2.Receptacle2_C"))
          (`/Game/DynamicGravityCharacter/Blueprints/Collectable_Receptacle/Receptacle2.SwitchToCharacter` _returnvalue_4))))))

(fn `UserConstructionScript`)