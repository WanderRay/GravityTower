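; SuccessBox5 is a trigger box that opens ShojiDoor6 when something begins overlapping its collision.
; The overlap calls OuvrirLesPortes, which sets the Ouverture flag, then passes a DoOnce to play an unlock sound, start the door timeline and call CallCameraToRoom4.
; The timeline adds a lerped offset to the door's current Y position on each update, so the slide accumulates instead of interpolating between fixed endpoints.
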(event `self.Collision.OnComponentBeginOverlap`
  (params (OverlappedComponent :type "PrimitiveComponent Object Reference") (OtherActor :type "Actor Object Reference") (OtherComp :type "PrimitiveComponent Object Reference") (OtherBodyIndex :type Integer) (bFromSweep :type Boolean) (SweepResult :type "HitResult Structure (by ref)"))
  ;[1 1 1] Le successbox 2 a besoin d'être dans le level il faut donc le cacher
  (`self.OuvrirLesPortes`))

(event `OuvrirLesPortes`
  ;[1 1 1] Le successbox 2 a besoin d'être dans le level il faut donc le cacher
  (set `self.Ouverture` true)
  (`/Engine/EditorBlueprintResources/StandardMacros.DoOnce` false
    (:`Completed`
      (`|ExecutionSequence`
        (:`then_0`
          (`GameplayStatics.PlaySound2D` "/Game/DynamicGravityCharacter/SFX/UnlockingSpecialNote.UnlockingSpecialNote" 1.0 1.0 0.0 null null)
          (`|ExecutionSequence`
            (:`then_0`
              (bind _returnvalue (`GameplayStatics.GetActorOfClass` "/Game/DynamicGravityCharacter/Blueprints/ZonesInteractions/ShojiDoor/ShojiDoor6.ShojiDoor6_C"))
              (bind (_direction _1_0) (`Timeline|Timeline_0` :!via `PlayFromStart`)
                (:`Update`
                  (bind (_returnvalue_x _returnvalue_y _returnvalue_z) (`KismetMathLibrary.BreakVector` (`self.K2_GetActorLocation` _returnvalue)))
                  (`self.K2_SetActorLocation` _returnvalue (`KismetMathLibrary.MakeVector` _returnvalue_x (+ (`KismetMathLibrary.Lerp` 0.0 6.0 _1_0) _returnvalue_y) _returnvalue_z) false false))))))
        (:`then_1`
          (`self.CameraToRoom4`))))))

(event `self.Collision.OnComponentEndOverlap`
  (params (OverlappedComponent :type "PrimitiveComponent Object Reference") (OtherActor :type "Actor Object Reference") (OtherComp :type "PrimitiveComponent Object Reference") (OtherBodyIndex :type Integer)))

(fn `UserConstructionScript`)