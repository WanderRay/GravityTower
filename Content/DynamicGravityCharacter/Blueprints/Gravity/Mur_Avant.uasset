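; Gravity field actor (Mur_Avant) that feeds custom gravity to dynamic-gravity characters overlapping it.
; Overlaps maintain the actor list, stop entering Characters' jumps, and switch Tick off once the field empties.
; Tick adds each enabled point, directional or line-based impulse, divided by delta time, to the character's DynGrav.
; All modes affect DGCharacterBP, but only directional gravity also handles DGCharacterBP1.
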(event `self.ReceiveActorBeginOverlap`
  (params (OtherActor :type "Actor Object Reference"))
  (`|ExecutionSequence`
    (:`then_1`
      (`self.AddActorToTheField` OtherActor)
      (`|ExecutionSequence`
        (:`then_0`
          (bind _ascharacter (cast `Character` OtherActor))
          (`Character.StopJumping` _ascharacter))
        (:`then_1`
          (cast `/Game/DynamicGravityCharacter/Blueprints/Character+MovingWalls/DGCharacterBP1` OtherActor))))))

(event `self.ReceiveActorEndOverlap`
  (params (OtherActor :type "Actor Object Reference"))
  (`self.RemoveActorFromTheField` OtherActor))

(event `self.ReceiveTick`
  (params (DeltaSeconds :type "Float (single-precision)"))
  (for _array_element (`self.ActorsInTheField`)
    (if (`self.EnablePointGravity`)
      (`self.ApplyPointImpulseToTheActor` _array_element))
    (if (`self.EnableDirectionalGravity`)
      (`self.ApplyDirectionalImpulseToTheActor` _array_element))
    (if (`self.EnableLinearGravity`)
      (`self.ApplyLinearImpulseToTheActor` _array_element))))

(fn `AddActorToTheField`
  (params (Actor :type "Actor Object Reference"))
  (returns (Index :type Integer))
  (bind _returnvalue (`KismetArrayLibrary.Array_Add` (`self.ActorsInTheField`) Actor))
  (`self.SetActorTickEnabled` true)
  (return _returnvalue))

(fn `ApplyDirectionalImpulseToTheActor`
  (params (Actor :type "Actor Object Reference"))
  (`|ExecutionSequence`
    (:`then_0`
      (bind _asdgcharacter_bp (cast `/Game/DynamicGravityCharacter/Blueprints/Character+MovingWalls/DGCharacterBP` Actor))
      (set `/Game/DynamicGravityCharacter/Blueprints/Character+MovingWalls/DGCharacterBP.DynGrav` (+ (/ (`self.DirectionalImpulse`) (`GameplayStatics.GetWorldDeltaSeconds`)) (`/Game/DynamicGravityCharacter/Blueprints/Character+MovingWalls/DGCharacterBP.DynGrav` _asdgcharacter_bp)) _asdgcharacter_bp))
    (:`then_1`
      (bind _asdgcharacter_bp1 (cast `/Game/DynamicGravityCharacter/Blueprints/Character+MovingWalls/DGCharacterBP1` Actor))
      (set `/Game/DynamicGravityCharacter/Blueprints/Character+MovingWalls/DGCharacterBP1.DynGrav` (+ (/ (`self.DirectionalImpulse`) (`GameplayStatics.GetWorldDeltaSeconds`)) (`/Game/DynamicGravityCharacter/Blueprints/Character+MovingWalls/DGCharacterBP1.DynGrav` _asdgcharacter_bp1)) _asdgcharacter_bp1))))

(fn `ApplyLinearImpulseToTheActor`
  (params (Actor :type "Actor Object Reference"))
  (bind _returnvalue (`KismetMathLibrary.GreaterGreater_VectorRotator` (`self.GravityLine`) (`self.K2_GetActorRotation`)))
  (bind _asdgcharacter_bp (cast `/Game/DynamicGravityCharacter/Blueprints/Character+MovingWalls/DGCharacterBP` Actor))
  (set `/Game/DynamicGravityCharacter/Blueprints/Character+MovingWalls/DGCharacterBP.DynGrav` (+ (* (`KismetMathLibrary.Normal` (`KismetMathLibrary.RotateAngleAxis` (`KismetMathLibrary.Cross_VectorVector` (- (`self.K2_GetActorLocation`) (`self.K2_GetActorLocation` Actor)) _returnvalue) 90.0 _returnvalue)) (/ (`self.LinearImpulse`) (`GameplayStatics.GetWorldDeltaSeconds`))) (`/Game/DynamicGravityCharacter/Blueprints/Character+MovingWalls/DGCharacterBP.DynGrav` _asdgcharacter_bp)) _asdgcharacter_bp))

(fn `ApplyPointImpulseToTheActor`
  (params (Actor :type "Actor Object Reference"))
  (`|ExecutionSequence`
    (:`then_0`
      (bind _asdgcharacter_bp (cast `/Game/DynamicGravityCharacter/Blueprints/Character+MovingWalls/DGCharacterBP` Actor))
      (set `/Game/DynamicGravityCharacter/Blueprints/Character+MovingWalls/DGCharacterBP.DynGrav` (+ (* (`KismetMathLibrary.Normal` (- (+ (`self.K2_GetActorLocation`) (`self.GravityCenter`)) (`self.K2_GetActorLocation` _asdgcharacter_bp))) (/ (`self.PointGravityImpulse`) (`GameplayStatics.GetWorldDeltaSeconds`))) (`/Game/DynamicGravityCharacter/Blueprints/Character+MovingWalls/DGCharacterBP.DynGrav` _asdgcharacter_bp)) _asdgcharacter_bp))))

(fn `RemoveActorFromTheField`
  (params (Actor :type "Actor Object Reference"))
  (returns (ActorRemoved :type Boolean))
  (bind _actorsinthefield (`self.ActorsInTheField`))
  (bind _returnvalue (`KismetArrayLibrary.Array_RemoveItem` _actorsinthefield Actor))
  (if (<= (`KismetArrayLibrary.Array_Length` _actorsinthefield) 0)
    (`self.SetActorTickEnabled` false))
  (return _returnvalue))

(fn `UserConstructionScript`)