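; ShieldProjectile is a projectile actor in the Dynamic Gravity character project that drives its own yaw rotation.
; Each Tick applies a stored yaw, provided the player pawn is a DGCharacterBP, then a one-second Delay clears the Ouvert flag.
; While Ouvert is set, the yaw grows by a fixed step per frame, so the spin is frame-rate dependent.
; A line trace and a MaxSpeed setter are left unconnected.
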(event `self.ReceiveTick`
  (params (DeltaSeconds :type "Float (single-precision)"))
  (`|ExecutionSequence`
    (:`then_0`
      (cast `/Game/DynamicGravityCharacter/Blueprints/Character+MovingWalls/DGCharacterBP` (`GameplayStatics.GetPlayerPawn` 0))
      (`self.K2_SetActorRotation` (`KismetMathLibrary.MakeRotator` 0.0 0.0 (`self.+1`)))
      (`KismetSystemLibrary.Delay` 1.0)
      (set `self.Ouvert` false))
    (:`then_1`
      (if (`self.Ouvert`)
        (set `self.+1` (+ (`self.+1`) 5.0))))))

(fn `UserConstructionScript`)