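; Character Blueprint for a dynamic-gravity pawn that updates its gravity and orientation settings every Tick.
; It passes DynGrav to the DGCharacterMovementComponent, then zeroes it, so the value must be refreshed each frame.
; Walkable floor normal follows the floor impact while walking and moving; otherwise it follows gravity and view rotation base is set to vertical direction.
; Tick also forces actor rotation to zero; some disconnected location-setting nodes remain unused.
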(event `self.ReceiveTick`
  (params (DeltaSeconds :type "Float (single-precision)"))
  ;[1 1 1] Tick
  (`|ExecutionSequence`
    (:`then_0`
      (bind _asdgcharacter_movement_component (cast `DGCharacterMovementComponent` (`self.CharacterMovement`)))
      (set `DGCharacterMovementComponent.DynamicGravity` (`self.DynGrav`) _asdgcharacter_movement_component)
      (set `self.DynGrav` (0.0 0.0 0.0))
      (if (and (`CharacterMovementComponent.IsWalking` (`self.CharacterMovement`)) (!= (`self.GetVelocity`) (0.0 0.0 0.0)))
        (set `DGCharacterMovementComponent.WalkableFloorNormalMode` "WFN_FloorImpactNormal" _asdgcharacter_movement_component)
        (else
          (set `DGCharacterMovementComponent.WalkableFloorNormalMode` "WFN_Gravity" _asdgcharacter_movement_component)
          (set `self.ViewRotationBaseMode` "VRM_VerticalDirection"))))
    (:`then_1`
      (`self.K2_SetActorRotation` (struct)))))

(fn `UserConstructionScript`)