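; Receptacle actor where the player character deposits carried collectables until a required count is reached.
; When a DGCharacterBP carrying a collectable overlaps the box, it clears the carried flag and visual, plays sounds and increments the count.
; Tick checks the count against the target, then once spawns a Receptacle3_3Vide at its transform and destroys its own mesh and box components.
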(event `self.Box.OnComponentBeginOverlap`
  (params (OverlappedComponent :type "PrimitiveComponent Object Reference") (OtherActor :type "Actor Object Reference") (OtherComp :type "PrimitiveComponent Object Reference") (OtherBodyIndex :type Integer) (bFromSweep :type Boolean) (SweepResult :type "HitResult Structure (by ref)"))
  (bind _asdgcharacter_bp (cast `/Game/DynamicGravityCharacter/Blueprints/Character+MovingWalls/DGCharacterBP` OtherActor))
  (if (`/Game/DynamicGravityCharacter/Blueprints/Character+MovingWalls/DGCharacterBP.CollectableOn` _asdgcharacter_bp)
    (set `/Game/DynamicGravityCharacter/Blueprints/Character+MovingWalls/DGCharacterBP.CollectableOn` false _asdgcharacter_bp)
    (`|ExecutionSequence`
      (:`then_0`
        (`GameplayStatics.PlaySound2D` "/Game/DynamicGravityCharacter/SFX/Fire.Fire" 1.0 1.0 0.0 null null))
      (:`then_1`
        (`GameplayStatics.PlaySound2D` "/Game/DynamicGravityCharacter/SFX/2SecondNote.2SecondNote" 1.0 1.0 0.0 null null)
        (bind _collectable (`/Game/DynamicGravityCharacter/Blueprints/Character+MovingWalls/DGCharacterBP.Collectable` _asdgcharacter_bp))
        (`StaticMeshComponent.SetStaticMesh` _collectable "/Game/DynamicGravityCharacter/FBX/None1/None1.None1")
        (`PrimitiveComponent.SetMaterial` _collectable 0 "/Game/DynamicGravityCharacter/FBX/None1/Translucent.Translucent"))
      (:`then_2`
        (set `self.Collected` (+ (`self.Collected`) 1.0))))))

(event `self.ReceiveTick`
  (params (DeltaSeconds :type "Float (single-precision)"))
  (if (>= (`self.Collected`) (`self.NumberOfObjetToCollect`))
    (`/Engine/EditorBlueprintResources/StandardMacros.DoOnce` false
      (:`Completed`
        (`|SpawnActorFromClass` "/Game/DynamicGravityCharacter/Blueprints/Collectable_Receptacle/Receptacle3_3Vide.Receptacle3_3Vide_C" (`SceneComponent.K2_GetComponentToWorld` (`self.DefaultSceneRoot`)) "Undefined" "OverrideRootScale" null null)
        (`ActorComponent.K2_DestroyComponent` (`self.StaticMesh`))
        (`ActorComponent.K2_DestroyComponent` (`self.Box`))))))

(fn `UserConstructionScript`)