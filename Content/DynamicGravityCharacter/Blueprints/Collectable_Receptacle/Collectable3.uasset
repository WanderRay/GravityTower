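; Collectable3 is a pickup actor for the Room 3 collectable, carried by the DGCharacterBP player character.
; A sphere overlap picks it up only if the character's CollectableOn flag is false, limiting the player to one at a time.
; Pickup plays a note sound, destroys the actor, sets the flag and shows a yellow cube on the character's Collectable mesh.
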(event `self.ReceiveBeginPlay`
  (set `self.CollectableRoom3` "Room3"))

(event `self.Sphere.OnComponentBeginOverlap`
  (params (OverlappedComponent :type "PrimitiveComponent Object Reference") (OtherActor :type "Actor Object Reference") (OtherComp :type "PrimitiveComponent Object Reference") (OtherBodyIndex :type Integer) (bFromSweep :type Boolean) (SweepResult :type "HitResult Structure (by ref)"))
  (bind _asdgcharacter_bp (cast `/Game/DynamicGravityCharacter/Blueprints/Character+MovingWalls/DGCharacterBP` OtherActor))
  (if (not (`/Game/DynamicGravityCharacter/Blueprints/Character+MovingWalls/DGCharacterBP.CollectableOn` _asdgcharacter_bp))
    (`|ExecutionSequence`
      (:`then_0`
        (`GameplayStatics.PlaySound2D` "/Game/DynamicGravityCharacter/SFX/1Firstnote.1Firstnote" 1.0 1.0 0.0 null null)
        (`self.K2_DestroyActor`)
        (set `/Game/DynamicGravityCharacter/Blueprints/Character+MovingWalls/DGCharacterBP.CollectableOn` true _asdgcharacter_bp)
        (bind _collectable (`/Game/DynamicGravityCharacter/Blueprints/Character+MovingWalls/DGCharacterBP.Collectable` _asdgcharacter_bp))
        (`StaticMeshComponent.SetStaticMesh` _collectable "/Game/Geometry/Meshes/1M_Cube.1M_Cube")
        (`PrimitiveComponent.SetMaterial` _collectable 0 "/Game/DynamicGravityCharacter/Materials/Yellow.Yellow")))))

(fn `UserConstructionScript`)